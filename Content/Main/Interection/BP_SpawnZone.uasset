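; BP_SpawnZone is a box-shaped zone that scatters randomly chosen actors inside itself when play begins.
; BeginPlay loops to spawn from two class options at random points within the Box bounds, adjusting for collisions or skipping blocked spawns.
; Disconnected logic, which never runs, traces from the Box to room Blueprints and mirrors their visibility onto the zone.
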(event EventBeginPlay
  (bind _box (Variables|Default|GetBox))
  (for _index (range 0 5)
    (Game|SpawnActorfromClass (Utilities|Array|Get(acopy) (Variables|Default|GetClass) (Math|Random|RandomIntegerinRange 0 1)) (Math|Conversions|ToTransform(Vector) (Math|Random|RandomPointinBoundingBox (Transformation|GetWorldLocation _box) (Components|Box|GetScaledBoxExtent _box))) "AdjustIfPossibleButDontSpawnIfColliding" 0 0)))

(event Collision|EventActorBeginOverlap
  (params (OtherActor :type Actor%20Object%20Reference)))

(event EventTick
  (params (DeltaSeconds :type Float%20%28single-precision%29)))

(fn ConstructionScript)