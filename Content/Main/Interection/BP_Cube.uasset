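; BP_Cube is a cube actor that picks a random material at BeginPlay and mirrors the visibility of a traced room.
; Every Tick, unless OnChar is set, it line-traces from its Arrow, multiplying rather than adding location for the end point.
; Sequenced casts to BP_RoomMain and Rooms 2–4 copy the hit room's Visible flag to the cube.
; While OnChar is true, it disables cube collision instead.
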(event EventBeginPlay
  (CallFunction|SetMaterial)
  (Rendering|SetVisibility (Variables|Default|GetCube) true false)
  (Variables|Default|SetOnChar false))

(event Collision|EventActorBeginOverlap
  (params (OtherActor :type Actor%20Object%20Reference)))

(event EventTick
  (params (DeltaSeconds :type Float%20%28single-precision%29))
  (bind _arrow (Variables|Default|GetArrow))
  (bind _returnvalue (Transformation|GetWorldLocation _arrow))
  (if (Variables|Default|GetOnChar)
    (Collision|SetCollisionEnabled (Variables|Default|GetCube) "NoCollision")
    (else
      (bind _outhit (Collision|LineTraceByChannel _returnvalue (* (* (Math|Vector|GetForwardVector _arrow) 1e+02) _returnvalue) "TraceTypeQuery2" false (Utilities|Array|MakeArray (Variables|Default|GetBP_Sphere) 0) "None"))
      (Utilities|FlowControl|Sequence
        (:then_0
          (bind _asbp_room_main (Utilities|Casting|CastToBP_RoomMain (.HitActor (Collision|BreakHitResult _outhit))))
          (bind _output_get (Variables|Default|SetAs%20BP%20Room%20Main _asbp_room_main))
          (if (Variables|/Game/Main/Room/BP_RoomMain.BP_RoomMain_C|GetVisible _output_get)
            (Rendering|SetVisibility (Variables|Default|GetCube) true false)
            (else
              (Rendering|SetVisibility (Variables|Default|GetCube) false false)
              (Variables|Default|SetAs%20BP%20Room%20Main 0))))
        (:then_1
          (bind _asbp_room_2 (Utilities|Casting|CastToBP_Room2 (.HitActor (Collision|BreakHitResult _outhit))))
          (bind _output_get_2 (Variables|Default|SetAs%20BP%20Room%202 _asbp_room_2))
          (if (Variables|/Game/Main/Room/BP_Room2.BP_Room2_C|GetVisible _output_get_2)
            (Rendering|SetVisibility (Variables|Default|GetCube) true false)
            (else
              (Rendering|SetVisibility (Variables|Default|GetCube) false false)
              (Variables|Default|SetAs%20BP%20Room%202 0))))
        (:then_2
          (bind _asbp_room_3 (Utilities|Casting|CastToBP_Room3 (.HitActor (Collision|BreakHitResult _outhit))))
          (bind _output_get_3 (Variables|Default|SetAs%20BP%20Room%203 _asbp_room_3))
          (if (Variables|/Game/Main/Room/BP_Room3.BP_Room3_C|GetVisible _output_get_3)
            (Rendering|SetVisibility (Variables|Default|GetCube) true false)
            (else
              (Rendering|SetVisibility (Variables|Default|GetCube) false false)
              (Variables|Default|SetAs%20BP%20Room%203 0))))
        (:then_3
          (bind _asbp_room_4 (Utilities|Casting|CastToBP_Room4 (.HitActor (Collision|BreakHitResult _outhit))))
          (bind _output_get_4 (Variables|Default|SetAs%20BP%20Room%204 _asbp_room_4))
          (if (Variables|/Game/Main/Room/BP_Room4.BP_Room4_C|GetVisible _output_get_4)
            (Rendering|SetVisibility (Variables|Default|GetCube) true false)
            (else
              (Rendering|SetVisibility (Variables|Default|GetCube) false false)
              (Variables|Default|SetAs%20BP%20Room%204 0))))))))

(fn ConstructionScript)

(fn SetMaterial
  (bind _material (Variables|Default|GetMaterial))
  (Rendering|Material|SetMaterial (Variables|Default|GetCube) 0 (Utilities|Array|Get(acopy) _material (Math|Random|RandomInteger (+ (Utilities|Array|LastIndex _material) 1)))))