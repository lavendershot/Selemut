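; BP_BI_Sphere is an interactable sphere actor that gets a randomized look and can be destroyed through interaction.
; On BeginPlay it sets an entry from its Material array on a material slot of the Sphere, randomizing both slot index and material choice.
; The ActivateInteract event stores its flag as Available and passes it to the DestroyActor function, which destroys the actor when true.
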(event EventBeginPlay
  (bind _returnvalue (Math|Random|RandomIntegerinRange 0 2))
  (Rendering|Material|SetMaterial (Variables|Default|GetSphere) _returnvalue (Utilities|Array|Get(acopy) (Variables|Default|GetMaterial) _returnvalue)))

(event Collision|EventActorBeginOverlap
  (params (OtherActor :type Actor%20Object%20Reference)))

(event EventTick
  (params (DeltaSeconds :type Float%20%28single-precision%29)))

(event EventActivateInteract
  (params (ActivateInteract :type Boolean))
  (bind _output_get (Variables|Default|SetActivate%20Interact ActivateInteract))
  (Variables|Default|SetAvailable _output_get)
  (CallFunction|DestroyActor (Variables|Default|GetAvailable)))

(fn ConstructionScript
  (|CallParentFunction))

(fn DestroyActor
  (params (Available :type Boolean))
  (Variables|Default|SetAvailable Available)
  (if (Variables|Default|GetAvailable)
    (Actor|DestroyActor)))