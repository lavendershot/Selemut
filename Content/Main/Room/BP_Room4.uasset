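; BP_Room4 is a room actor that shows its walls, floor and stairs only while the player is inside its trigger box.
; BeginPlay gathers those components into the SMVisibility array, hides them and clears the Visible flag.
; Box begin and end overlap events filter for player pawn 0, then toggle the components' visibility without propagating to children and update Visible to match.
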(event OnComponentBeginOverlap(Box)
  (params (OverlappedComponent :type Primitive%20Component%20Object%20Reference) (OtherActor :type Actor%20Object%20Reference) (OtherComp :type Primitive%20Component%20Object%20Reference) (OtherBodyIndex :type Integer) (bFromSweep :type Boolean) (SweepResult :type Hit%20Result%20Structure%20%28by%20ref%29))
  (if (== OtherActor (Game|Player|GetPlayerPawn 0))
    (Rendering|SetVisibility (Variables|Default|GetSM_Visibility) true false)
    (Variables|Default|SetVisible true)))

(event OnComponentEndOverlap(Box)
  (params (OverlappedComponent :type Primitive%20Component%20Object%20Reference) (OtherActor :type Actor%20Object%20Reference) (OtherComp :type Primitive%20Component%20Object%20Reference) (OtherBodyIndex :type Integer))
  (if (== OtherActor (Game|Player|GetPlayerPawn 0))
    (Rendering|SetVisibility (Variables|Default|GetSM_Visibility) false false)
    (Variables|Default|SetVisible false)))

(event EventBeginPlay
  (bind _output_get (Variables|Default|SetSM_Visibility (Utilities|Array|MakeArray (Variables|Default|GetWall1) (Variables|Default|GetWall2.1) (Variables|Default|GetWall2) (Variables|Default|GetFloor) (Variables|Default|GetStairs1))))
  (Rendering|SetVisibility _output_get false false)
  (Variables|Default|SetVisible false))

(event Collision|EventActorBeginOverlap
  (params (OtherActor :type Actor%20Object%20Reference)))

(event EventTick
  (params (DeltaSeconds :type Float%20%28single-precision%29)))

(fn ConstructionScript)